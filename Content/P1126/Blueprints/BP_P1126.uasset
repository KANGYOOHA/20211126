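; BP_P1126 is an actor that moves steadily along the world X axis while spinning its Left and Right components.
; Each Tick calls P1126MoveForward, which scales SecondSpeed by delta time and applies it as local roll to both components.
; The actor offset uses a hardcoded frame-rate-independent speed, so travel is independent of SecondSpeed and of the actor's facing.
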(event `self.ReceiveTick`
  (params (DeltaSeconds :type "Float (single-precision)"))
  (`self.P1126MoveForward`))

(fn `P1126MoveForward`
  (set `self.FrameSpeed` (* (`GameplayStatics.GetWorldDeltaSeconds`) (`self.SecondSpeed`)))
  (`SceneComponent.K2_AddLocalRotation` (`self.Left`) (`KismetMathLibrary.MakeRotator` (`self.FrameSpeed`)) false false)
  (`SceneComponent.K2_AddLocalRotation` (`self.Right`) (`KismetMathLibrary.MakeRotator` (`self.FrameSpeed`)) false false)
  (`self.K2_AddActorWorldOffset` (`KismetMathLibrary.MakeVector` (* (`GameplayStatics.GetWorldDeltaSeconds`) 100.0))))

(fn `UserConstructionScript`)